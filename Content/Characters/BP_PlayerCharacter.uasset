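; Player character for a maze game, handling movement, look, jump, sprint, damage and pause input.
; Grounded movement triggers camera shake and footstep sounds, throttled by a DoOnce whose reset delay shortens while SprintComponent reports sprinting.
; Damage lowers Health, refreshes the HUD and triggers the loss through MazeGameMode, which also handles pausing.
; Outside debug mode, the first key press swaps the loading screen for the HUD, restores game input and starts music.
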(event `InputAxis|MoveForward`
  (params (AxisValue :type "Float (single-precision)"))
  (bind _returnvalue (`GameplayStatics.GetPlayerController` 0))
  ;[1 1 1] Movement handling
  (`self.AddMovementInput` (`self.GetActorForwardVector`) AxisValue)
  (if (`NavMovementComponent.IsMovingOnGround` (`self.CharacterMovement`))
    (`PlayerController.ClientStartCameraShake` :`self` _returnvalue :`Shake` (`self.CameraShakeClass`) :`Scale` (`KismetMathLibrary.FClamp` (`KismetMathLibrary.Abs` AxisValue)))
    (`PlayerController.ClientStopCameraShake` _returnvalue (`self.CameraShakeClass`) false)
    (if (!= AxisValue 0.0)
      (`/Engine/EditorBlueprintResources/StandardMacros.DoOnce` false :!label _label
        (:`Completed`
          (`GameplayStatics.PlaySoundAtLocation` "/Game/Sounds/SFX/A_Footstep.A_Footstep" (`self.K2_GetActorLocation`) (struct) 1.0 1.0 0.0 null null null)
          (if (`/Game/Blueprints/ActorComponents/BP_SprintComponent.IsSprinting` (`self.SprintComponent`))
            (`KismetSystemLibrary.Delay` 0.3)
            (goto _label :!via `Reset`)
            (else
              (`KismetSystemLibrary.Delay` 0.5)
              (goto _label :!via `Reset`))))))))

(event `InputAxis|MoveRight`
  (params (AxisValue :type "Float (single-precision)"))
  (bind _returnvalue (`GameplayStatics.GetPlayerController` 0))
  ;[1 1 1] Movement handling
  (`self.AddMovementInput` (`self.GetActorRightVector`) AxisValue)
  (if (`NavMovementComponent.IsMovingOnGround` (`self.CharacterMovement`))
    (`PlayerController.ClientStartCameraShake` :`self` _returnvalue :`Shake` (`self.CameraShakeClass`) :`Scale` (`KismetMathLibrary.FClamp` (`KismetMathLibrary.Abs` AxisValue)))
    (`PlayerController.ClientStopCameraShake` _returnvalue (`self.CameraShakeClass`) false)
    (if (!= AxisValue 0.0)
      (goto _label))))

(event `InputAxis|Turn`
  (params (AxisValue :type "Float (single-precision)"))
  ;[1 1 1] Movement handling
  (`self.AddControllerYawInput` AxisValue))

(event `InputAxis|LookUp`
  (params (AxisValue :type "Float (single-precision)"))
  ;[1 1 1] Movement handling
  (`self.AddControllerPitchInput` AxisValue))

(event `InputAction|Jump`
  (params (Key :type "Key Structure"))
  ;[1 1 1] Movement handling
  (:`Pressed`
    (`self.Jump`))
  (:`Released`
    (`self.StopJumping`)))

(event `InputAction|Sprint`
  (params (Key :type "Key Structure"))
  (bind _sprintcomponent (`self.SprintComponent`))
  ;[1 1 1] Movement handling
  (:`Pressed`
    (`/Game/Blueprints/ActorComponents/BP_SprintComponent.OnSprint` _sprintcomponent))
  (:`Released`
    (`/Game/Blueprints/ActorComponents/BP_SprintComponent.OnWalk` _sprintcomponent)))

(event `self.ReceiveAnyDamage`
  (params (Damage :type "Float (single-precision)") (DamageType :type "DamageType Object Reference") (InstigatedBy :type "Controller Object Reference") (DamageCauser :type "Actor Object Reference"))
  ;[1 1 1] Damage handling
  (`|ExecutionSequence`
    (:`then_0`
      (set `self.Health` (- (`self.Health`) (`KismetMathLibrary.FTrunc` Damage)))
      (bind _asmaze_game_mode (cast `/Game/Core/GameModes/MazeGameMode` (`GameplayStatics.GetGameMode`)))
      (bind _headsupdisplay (`/Game/Core/GameModes/MazeGameMode.HeadsUpDisplay` _asmaze_game_mode)
        (:`then`
          (`/Game/UI/WBP_HeadsUpDisplay.OnUpdateHealth` _headsupdisplay))
        (:`else`)))
    (:`then_1`
      (if (<= (`self.Health`) 0)
        (`/Game/Core/GameModes/MazeGameMode.OnLose` _asmaze_game_mode)))))

(event `InputAction|TogglePauseMenu` :paused true
  (params (Key :type "Key Structure"))
  ;[1 1 1] Toggle pause menu
  (:`Pressed`
    (bind _asmaze_game_mode (cast `/Game/Core/GameModes/MazeGameMode` (`GameplayStatics.GetGameMode`)))
    (if (`GameplayStatics.IsGamePaused`)
      (`/Game/Core/GameModes/MazeGameMode.OnResumeGame` _asmaze_game_mode)
      (else
        (`/Game/Core/GameModes/MazeGameMode.OnPauseGame` _asmaze_game_mode)))))

(event `Key|AnyKey`
  (params (Key :type "Key Structure"))
  (bind _returnvalue (`GameplayStatics.GetPlayerController` 0))
  ;[1 1 1] Loading screen handling
  (:`Pressed`
    (bind _asmaze_game_mode (cast `/Game/Core/GameModes/MazeGameMode` (`GameplayStatics.GetGameMode`)))
    (if (not (`/Game/Core/GameModes/MazeGameMode.IsDebuggingOn` _asmaze_game_mode))
      (`/Engine/EditorBlueprintResources/StandardMacros.DoOnce` false
        (:`Completed`
          (`Widget.RemoveFromParent` (`/Game/Core/GameModes/MazeGameMode.LoadingScreen` _asmaze_game_mode))
          (`WidgetBlueprintLibrary.SetInputMode_GameOnly` _returnvalue)
          (set `PlayerController.bShowMouseCursor` false _returnvalue)
          (`UserWidget.AddToViewport` (`/Game/Core/GameModes/MazeGameMode.HeadsUpDisplay` _asmaze_game_mode) 0)
          (`GameplayStatics.PlaySound2D` "/Game/Sounds/Music/A_LightlessDawn_Music.A_LightlessDawn_Music" 1.0 1.0 0.0 null null))))))

(fn `UserConstructionScript`)