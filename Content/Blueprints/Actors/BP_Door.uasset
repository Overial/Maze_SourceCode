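; Locked maze door that the player opens by spending a key, sliding the door mesh along Z.
; A trigger volume shows HUD prompts and enables Interact input only while a player holding a key overlaps it.
; Interact decrements the key count, attaches a key mesh at the keyhole, and plays a sound and timeline moving key and door.
; On BeginPlay, a door listed in the save game's OpenedDoors by display name starts open.
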(event `self.ReceiveBeginPlay`
  (bind _asmaze_game_instance (cast `/Game/Core/GameInstances/MazeGameInstance` (`GameplayStatics.GetGameInstance`)))
  (bind _returnvalue (`GameplayStatics.DoesSaveGameExist` (`/Game/Core/GameInstances/MazeGameInstance.SlotName` _asmaze_game_instance)))
  (if _returnvalue
    (bind _returnvalue_2 (`GameplayStatics.LoadGameFromSlot` (`/Game/Core/GameInstances/MazeGameInstance.SlotName` _asmaze_game_instance)))
    (bind _assave_game_object (cast `/Game/Core/SaveGameObjects/SaveGameObject` _returnvalue_2))
    (if (!= (`KismetArrayLibrary.Array_Find` (`/Game/Core/SaveGameObjects/SaveGameObject.OpenedDoors` _assave_game_object) (`KismetSystemLibrary.GetDisplayName` self)) -1)
      (`SceneComponent.K2_SetRelativeLocation` (`self.DoorMesh`) (0.0 0.0 -310.0) false false)
      (set `self.IsOpen` true))))

(event `self.TriggerVolume.OnComponentBeginOverlap`
  (params (OverlappedComponent :type "PrimitiveComponent Object Reference") (OtherActor :type "Actor Object Reference") (OtherComp :type "PrimitiveComponent Object Reference") (OtherBodyIndex :type Integer) (bFromSweep :type Boolean) (SweepResult :type "HitResult Structure (by ref)"))
  (if (== OtherActor (`GameplayStatics.GetPlayerCharacter` 0))
    (if (not (`self.IsOpen`))
      (bind _asbp_player_character (cast `/Game/Characters/BP_PlayerCharacter` (`GameplayStatics.GetPlayerCharacter` 0)))
      (if (> (`/Game/Characters/BP_PlayerCharacter.KeyAmount` _asbp_player_character) 0)
        (`self.EnableInput` (`GameplayStatics.GetPlayerController` 0))
        (bind _asmaze_game_mode (cast `/Game/Core/GameModes/MazeGameMode` (`GameplayStatics.GetGameMode`)))
        (bind _headsupdisplay (`/Game/Core/GameModes/MazeGameMode.HeadsUpDisplay` _asmaze_game_mode)
          (:`then`
            (set `/Game/UI/WBP_HeadsUpDisplay.MessageText` "Press E to use key" _headsupdisplay)
            (`/Game/UI/WBP_HeadsUpDisplay.OnUpdateMessage` _headsupdisplay))
          (:`else`))
        (else
          (bind _asmaze_game_mode_2 (cast `/Game/Core/GameModes/MazeGameMode` (`GameplayStatics.GetGameMode`)))
          (bind _headsupdisplay_2 (`/Game/Core/GameModes/MazeGameMode.HeadsUpDisplay` _asmaze_game_mode_2)
            (:`then`
              (set `/Game/UI/WBP_HeadsUpDisplay.MessageText` "You need a key to open the door" _headsupdisplay_2)
              (`/Game/UI/WBP_HeadsUpDisplay.OnUpdateMessage` _headsupdisplay_2))
            (:`else`)))))))

(event `self.TriggerVolume.OnComponentEndOverlap`
  (params (OverlappedComponent :type "PrimitiveComponent Object Reference") (OtherActor :type "Actor Object Reference") (OtherComp :type "PrimitiveComponent Object Reference") (OtherBodyIndex :type Integer))
  (if (== OtherActor (`GameplayStatics.GetPlayerCharacter` 0))
    (`self.DisableInput` (`GameplayStatics.GetPlayerController` 0))
    (bind _asmaze_game_mode (cast `/Game/Core/GameModes/MazeGameMode` (`GameplayStatics.GetGameMode`)))
    (bind _headsupdisplay (`/Game/Core/GameModes/MazeGameMode.HeadsUpDisplay` _asmaze_game_mode))
    (set `/Game/UI/WBP_HeadsUpDisplay.MessageText` "" _headsupdisplay)
    (`/Game/UI/WBP_HeadsUpDisplay.OnUpdateMessage` _headsupdisplay)))

(event `InputAction|Interact`
  (params (Key :type "Key Structure"))
  (:`Pressed`
    (bind _asbp_player_character (cast `/Game/Characters/BP_PlayerCharacter` (`GameplayStatics.GetPlayerCharacter` 0)))
    (bind _keyamount (`/Game/Characters/BP_PlayerCharacter.KeyAmount` _asbp_player_character))
    (if (> _keyamount 0)
      (if (not (`self.IsOpen`))
        (`|ExecutionSequence`
          (:`then_0`
            (`/Engine/EditorBlueprintResources/StandardMacros.DecrementInt` _keyamount
              (:`  `
                (bind _asmaze_game_mode (cast `/Game/Core/GameModes/MazeGameMode` (`GameplayStatics.GetGameMode`)))
                (`/Game/UI/WBP_HeadsUpDisplay.OnUpdateKeyAmount` (`/Game/Core/GameModes/MazeGameMode.HeadsUpDisplay` _asmaze_game_mode)))))
          (:`then_1`
            (set `self.IsOpen` true)
            (bind _asmaze_game_mode_2 (cast `/Game/Core/GameModes/MazeGameMode` (`GameplayStatics.GetGameMode`)))
            (bind _headsupdisplay (`/Game/Core/GameModes/MazeGameMode.HeadsUpDisplay` _asmaze_game_mode_2))
            (set `/Game/UI/WBP_HeadsUpDisplay.MessageText` "" _headsupdisplay)
            (`/Game/UI/WBP_HeadsUpDisplay.OnUpdateMessage` _headsupdisplay))
          (:`then_2`
            (bind _returnvalue (`AddComponent|NODE_AddStaticMeshComponent-1`))
            (set `self.KeyMesh` _returnvalue)
            (`SceneComponent.K2_AttachToComponent` (`self.KeyMesh`) (`self.Keyhole`) "None" "SnapToTarget" "SnapToTarget" "SnapToTarget" true)
            (`GameplayStatics.PlaySoundAtLocation` "/Game/Sounds/SFX/A_DoorOpening.A_DoorOpening" (`self.K2_GetActorLocation`) (struct) 1.0 1.0 0.0 null null null)
            (bind (_direction _doorposition _keyposition) (`Timeline|DoorOpening` :!via `PlayFromStart`)
              (:`Update`
                (`SceneComponent.K2_SetRelativeLocation` (`self.KeyMesh`) (`KismetMathLibrary.MakeVector` 0.0 _keyposition) false false)
                (`SceneComponent.K2_SetRelativeLocation` (`self.DoorMesh`) (`KismetMathLibrary.MakeVector` 0.0 0.0 _doorposition) false false)))))))))

(fn `UserConstructionScript`)