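; BP_ArrowShooter is a trap actor that fires BP_Arrow projectiles when a living player steps into its line of fire.
; Each tick a sphere trace from the Detector reaches along the ArrowSource's forward direction up to ShootingRange and checks for a BP_PlayerCharacter with health left.
; A DoOnce gate spawns the arrow with a shot sound, then resets after DeltaTime, acting as a cooldown.
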(event `self.ReceiveBeginPlay`
  ;[1 1 1] (Disabled) Shooting every delta seconds
)

(event `OnShootArrow`
  ;[1 1 1] Shooting arrow
  (`/Engine/EditorBlueprintResources/StandardMacros.DoOnce` false :!label _label
    (:`Completed`
      (`|SpawnActorFromClass` "/Game/Blueprints/Actors/BP_Arrow.BP_Arrow_C" (`SceneComponent.K2_GetComponentToWorld` (`self.ArrowSource`)) "Undefined" "OverrideRootScale" null null)
      (`GameplayStatics.PlaySoundAtLocation` "/Game/Sounds/SFX/A_ArrowShot.A_ArrowShot" (`self.K2_GetActorLocation`) (struct) 1.0 1.0 0.0 null null null)
      (`KismetSystemLibrary.Delay` (`self.DeltaTime`))
      (goto _label :!via `Reset`))))

(event `self.ReceiveTick`
  (params (DeltaSeconds :type "Float (single-precision)"))
  (bind _arrowsource (`self.ArrowSource`))
  ;[1 1 1] Detector logic
  (bind _outhit (`KismetSystemLibrary.SphereTraceSingle` (`SceneComponent.K2_GetComponentLocation` (`self.Detector`)) (+ (`SceneComponent.K2_GetComponentLocation` _arrowsource) (* (`KismetMathLibrary.GetForwardVector` (`SceneComponent.K2_GetComponentRotation` _arrowsource)) (`self.ShootingRange`))) 10.0 "TraceTypeQuery2"))
  (bind _asbp_player_character (cast `/Game/Characters/BP_PlayerCharacter` (`.HitActor` (`GameplayStatics.BreakHitResult` _outhit))))
  (if (> (`/Game/Characters/BP_PlayerCharacter.Health` _asbp_player_character) 0)
    (`self.OnShootArrow`)))

(fn `UserConstructionScript`)