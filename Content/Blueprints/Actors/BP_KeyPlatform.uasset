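; A maze pedestal actor holding a key that the player collects by pressing Interact.
; On BeginPlay it loads the save slot named by the game instance and removes the key mesh if its display name is among the picked-up keys.
; The trigger volume toggles input and the HUD prompt for the player.
; Pickup destroys the mesh, increments the player's key count, updates the HUD and plays a sound, without writing the save.
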(event `self.ReceiveBeginPlay`
  (bind _asmaze_game_instance (cast `/Game/Core/GameInstances/MazeGameInstance` (`GameplayStatics.GetGameInstance`)))
  (bind _returnvalue (`GameplayStatics.DoesSaveGameExist` (`/Game/Core/GameInstances/MazeGameInstance.SlotName` _asmaze_game_instance)))
  (if _returnvalue
    (bind _returnvalue_2 (`GameplayStatics.LoadGameFromSlot` (`/Game/Core/GameInstances/MazeGameInstance.SlotName` _asmaze_game_instance)))
    (bind _assave_game_object (cast `/Game/Core/SaveGameObjects/SaveGameObject` _returnvalue_2))
    (if (!= (`KismetArrayLibrary.Array_Find` (`/Game/Core/SaveGameObjects/SaveGameObject.PickedUpKeys` _assave_game_object) (`KismetSystemLibrary.GetDisplayName` self)) -1)
      (bind _keymesh (`self.KeyMesh`)
        (:`then`
          (`ActorComponent.K2_DestroyComponent` _keymesh)
          (set `self.IsEmpty` true))
        (:`else`)))))

(event `self.TriggerVolume.OnComponentBeginOverlap`
  (params (OverlappedComponent :type "PrimitiveComponent Object Reference") (OtherActor :type "Actor Object Reference") (OtherComp :type "PrimitiveComponent Object Reference") (OtherBodyIndex :type Integer) (bFromSweep :type Boolean) (SweepResult :type "HitResult Structure (by ref)"))
  (if (== OtherActor (`GameplayStatics.GetPlayerCharacter` 0))
    (`self.EnableInput` (`GameplayStatics.GetPlayerController` 0))
    (`/Engine/EditorBlueprintResources/StandardMacros.IsValid` (`self.KeyMesh`)
      (:`Is Valid`
        (bind _asmaze_game_mode (cast `/Game/Core/GameModes/MazeGameMode` (`GameplayStatics.GetGameMode`)))
        (bind _headsupdisplay (`/Game/Core/GameModes/MazeGameMode.HeadsUpDisplay` _asmaze_game_mode))
        (set `/Game/UI/WBP_HeadsUpDisplay.MessageText` "Press E to pick up the key" _headsupdisplay)
        (`/Game/UI/WBP_HeadsUpDisplay.OnUpdateMessage` _headsupdisplay)))))

(event `self.TriggerVolume.OnComponentEndOverlap`
  (params (OverlappedComponent :type "PrimitiveComponent Object Reference") (OtherActor :type "Actor Object Reference") (OtherComp :type "PrimitiveComponent Object Reference") (OtherBodyIndex :type Integer))
  (if (== OtherActor (`GameplayStatics.GetPlayerCharacter` 0))
    (`self.DisableInput` (`GameplayStatics.GetPlayerController` 0))
    (bind _asmaze_game_mode (cast `/Game/Core/GameModes/MazeGameMode` (`GameplayStatics.GetGameMode`)))
    (bind _headsupdisplay (`/Game/Core/GameModes/MazeGameMode.HeadsUpDisplay` _asmaze_game_mode))
    (set `/Game/UI/WBP_HeadsUpDisplay.MessageText` "" _headsupdisplay)
    (`/Game/UI/WBP_HeadsUpDisplay.OnUpdateMessage` _headsupdisplay)))

(event `InputAction|Interact`
  (params (Key :type "Key Structure"))
  (:`Pressed`
    (bind _keymesh (`self.KeyMesh`)
      (:`then`
        (`ActorComponent.K2_DestroyComponent` _keymesh)
        (set `self.IsEmpty` true)
        (bind _asbp_player_character (cast `/Game/Characters/BP_PlayerCharacter` (`GameplayStatics.GetPlayerCharacter` 0)))
        (`/Engine/EditorBlueprintResources/StandardMacros.IncrementInt` (`/Game/Characters/BP_PlayerCharacter.KeyAmount` _asbp_player_character)
          (:`  `
            (bind _asmaze_game_mode (cast `/Game/Core/GameModes/MazeGameMode` (`GameplayStatics.GetGameMode`)))
            (`/Game/UI/WBP_HeadsUpDisplay.OnUpdateKeys` (`/Game/Core/GameModes/MazeGameMode.HeadsUpDisplay` _asmaze_game_mode))
            (bind _asmaze_game_mode_2 (cast `/Game/Core/GameModes/MazeGameMode` (`GameplayStatics.GetGameMode`)))
            (bind _headsupdisplay (`/Game/Core/GameModes/MazeGameMode.HeadsUpDisplay` _asmaze_game_mode_2))
            (set `/Game/UI/WBP_HeadsUpDisplay.MessageText` "" _headsupdisplay)
            (`/Game/UI/WBP_HeadsUpDisplay.OnUpdateMessage` _headsupdisplay)
            (`GameplayStatics.PlaySound2D` "/Game/Sounds/SFX/A_PickupKey.A_PickupKey" 1.0 1.0 0.0 null null))))
      (:`else`))))

(fn `UserConstructionScript`)