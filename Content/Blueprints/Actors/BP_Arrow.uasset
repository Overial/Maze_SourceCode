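; BP_Arrow is a projectile arrow that damages and knocks back the player character.
; Collision turns on just after spawn to avoid sticking at launch, while a timeline animates the mesh's pitch.
; Overlapping a living player while unstuck launches them along the arrow's velocity plus lift, applies damage, plays a sound and destroys the arrow.
; A blocking hit marks it stuck, stops rotation and destroys it after its lifetime.
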(event `self.ReceiveBeginPlay`
  (`|ExecutionSequence`
    (:`then_0`
      ;[1 1 1] Setting collision after launch (otherwise it will get stuck)
      (`KismetSystemLibrary.Delay` 0.01)
      (`PrimitiveComponent.SetCollisionEnabled` (`self.Sphere`) "QueryAndPhysics"))
    (:`then_1`
      ;[1 1 1] Setting looping rotation
      (bind (_direction _degrees) (`Timeline|ArrowRotation`)
        (:`Update`
          (`SceneComponent.K2_SetRelativeRotation` (`self.ArrowMesh`) (`KismetMathLibrary.MakeRotator` 0.0 _degrees -90.0) false false))))))

(event `self.Sphere.OnComponentBeginOverlap`
  (params (OverlappedComponent :type "PrimitiveComponent Object Reference") (OtherActor :type "Actor Object Reference") (OtherComp :type "PrimitiveComponent Object Reference") (OtherBodyIndex :type Integer) (bFromSweep :type Boolean) (SweepResult :type "HitResult Structure (by ref)"))
  ;[1 1 1] Hitting player character
  (if (not (`self.IsStuck`))
    (bind _asbp_player_character (cast `/Game/Characters/BP_PlayerCharacter` OtherActor))
    (if (> (`/Game/Characters/BP_PlayerCharacter.Health` _asbp_player_character) 0)
      (`Character.LaunchCharacter` _asbp_player_character (+ (`self.GetVelocity`) (0.0 0.0 200.0)) false false)
      (`GameplayStatics.ApplyDamage` _asbp_player_character (`self.BaseDamage`))
      (`self.K2_DestroyActor`)
      (`GameplayStatics.PlaySoundAtLocation` "/Game/Sounds/SFX/A_ArrowHit.A_ArrowHit" (`self.K2_GetActorLocation` (`GameplayStatics.GetPlayerCharacter` 0)) (struct) 1.0 1.0 0.0 null null null))))

(event `self.Sphere.OnComponentHit`
  (params (HitComponent :type "PrimitiveComponent Object Reference") (OtherActor :type "Actor Object Reference") (OtherComp :type "PrimitiveComponent Object Reference") (NormalImpulse :type "Vector Structure") (Hit :type "HitResult Structure (by ref)"))
  ;[1 1 1] Stopping arrow rotation when hit any object except player
  (set `self.IsStuck` true)
  (`TimelineComponent.Stop` (`self.ArrowRotation`))
  (`KismetSystemLibrary.Delay` (`self.Lifetime`))
  (`self.K2_DestroyActor`))

(fn `UserConstructionScript`)