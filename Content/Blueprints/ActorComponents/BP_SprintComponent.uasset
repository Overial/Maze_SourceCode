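; Actor component that toggles sprinting for the first player's character.
; OnSprint and OnWalk events set the character movement's max walk speed to the sprint or walk value and update the IsSprinting flag.
; Each event then casts that character to BP_PlayerCharacter and swaps its camera shake class between sprint and walk head bobbing.
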(event `OnSprint`
  (bind _returnvalue (`GameplayStatics.GetPlayerCharacter` 0))
  (set `CharacterMovementComponent.MaxWalkSpeed` (`self.SprintSpeed`) (`Character.CharacterMovement` _returnvalue))
  (set `self.IsSprinting` true)
  (bind _asbp_player_character (cast `/Game/Characters/BP_PlayerCharacter` _returnvalue))
  (set `/Game/Characters/BP_PlayerCharacter.CameraShakeClass` "/Game/Core/CameraShakeObjects/SprintHeadBobbing.SprintHeadBobbing_C" _asbp_player_character))

(event `OnWalk`
  (bind _returnvalue (`GameplayStatics.GetPlayerCharacter` 0))
  (set `CharacterMovementComponent.MaxWalkSpeed` (`self.WalkSpeed`) (`Character.CharacterMovement` _returnvalue))
  (set `self.IsSprinting` false)
  (bind _asbp_player_character (cast `/Game/Characters/BP_PlayerCharacter` _returnvalue))
  (set `/Game/Characters/BP_PlayerCharacter.CameraShakeClass` "/Game/Core/CameraShakeObjects/WalkHeadBobbing.WalkHeadBobbing_C" _asbp_player_character))